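; GA_Jump is a Gameplay Ability that makes the avatar Character jump.
; On activation it commits the ability, casts the avatar to Character and calls Jump if CanJump passes, ending at once if the commit or check fails.
; A WaitInputRelease task keeps the ability active until input is released, then calls StopJumping and ends it, with debug prints on release and end.
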(event `self.K2_ActivateAbility`
  (bind _returnvalue (`self.K2_CommitAbility`))
  (if _returnvalue
    (bind _ascharacter (cast `Character` (`self.GetAvatarActorFromActorInfo`)))
    (if (`Character.CanJump` _ascharacter)
      (`Character.Jump` _ascharacter)
      (`AbilityTask_WaitInputRelease.WaitInputRelease` true
        (:`OnRelease`
          (`Character.StopJumping` _ascharacter)
          (`KismetSystemLibrary.PrintString` "InputReleased")
          (`self.K2_EndAbility`)))
      (else
        (`self.K2_EndAbility`)))
    (else
      (`self.K2_EndAbility`))))

(event `self.K2_OnEndAbility`
  (params (bWasCancelled :type Boolean))
  (`KismetSystemLibrary.PrintString` "EndJump"))