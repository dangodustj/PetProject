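; Gameplay ability for a double jump that launches the avatar Character upward when activated.
; After a successful commit, it calls LaunchCharacter with the movement component's JumpZVelocity along up plus the last input vector, added to current velocity rather than overriding it.
; The ability ends immediately, also when the commit fails, and has no air or jump-count check of its own.
; A Jump and WaitInputRelease chain is left disconnected.
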(event `self.K2_ActivateAbility`
  (bind _returnvalue (`self.K2_CommitAbility`))
  (if _returnvalue
    (bind _ascharacter (cast `Character` (`self.GetAvatarActorFromActorInfo`)))
    (bind _charactermovement (`Character.CharacterMovement` _ascharacter))
    (`Character.LaunchCharacter` _ascharacter (+ (* (`CharacterMovementComponent.JumpZVelocity` _charactermovement) (`KismetMathLibrary.Vector_Up`)) (`PawnMovementComponent.GetLastInputVector` _charactermovement)) false false)
    (`self.K2_EndAbility`)
    (else
      (`self.K2_EndAbility`))))